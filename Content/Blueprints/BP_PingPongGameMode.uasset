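; Game mode for a two-team ping-pong match that tracks scores and match state across player controllers.
; OnBallScore increments a team score, checks the limit, naming the opposite team when one reaches it, and refreshes each pawn's score UI.
; StartMatch_Event sets every field player's match state.
; Player spawning, team assignment, ball spawn and removal, and win/lose handling exist only as disconnected logic, leaving EndMatch_Event, PlayerSpawned and GrandPlayerTag empty.
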(event `EndMatch_Event`
  (params (WinTeam :type Name)))

(event `CheckMatchRule`
  (if (== (`self.TeamScore2`) (`self.EndMacthScore`))
    (`self.EndMatch_Event` "Team1")
    (elif (== (`self.TeamScore1`) (`self.EndMacthScore`))
      (`self.EndMatch_Event` "Team2"))))

(event `StartMatch_Event`
  (for _array_element (`self.Controllers`)
    (bind _asbp_field_player_controller (cast `/Game/Blueprints/BP_FieldPlayerController` _array_element))
    (bind _asbp_field_player (cast `/Game/Blueprints/BP_FieldPlayer` (`Controller.K2_GetPawn` _asbp_field_player_controller)))
    (`/Game/Blueprints/BP_FieldPlayer.MatchState` _asbp_field_player 0)))

(event `OnBallScore`
  (params (ScoringTeam :type Integer))
  (switch `int` ScoringTeam
    (:`1`
      (`/Engine/EditorBlueprintResources/StandardMacros.IncrementInt` (`self.TeamScore1`)
        (:`  `
          _)))
    (:`2`
      (`/Engine/EditorBlueprintResources/StandardMacros.IncrementInt` (`self.TeamScore2`)
        (:`  `
          _))))
  (`self.CheckMatchRule`)
  (`self.Update_PlayerScoreUI`))

(event `PlayerSpawned`)

(event `GrandPlayerTag`)

(fn `Update_PlayerScoreUI`
  (for _array_element (`self.Controllers`)
    (bind _asbp_field_player (cast `/Game/Blueprints/BP_FieldPlayer` (`Controller.K2_GetPawn` _array_element)))
    (`/Game/Blueprints/BP_FieldPlayer.ChangeScore` _asbp_field_player (`self.TeamScore1`) (`self.TeamScore2`))))

(fn `UserConstructionScript`)