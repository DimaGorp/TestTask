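; BP_FieldPlayer is the player Blueprint in a ping pong game, linking match events to the HUD and game mode.
; Draw casts the controller's HUD to BP_HUD, caches it and draws the UI, then score and match-state events forward to that HUD.
; PlayerSpawned notifies BP_PingPongGameMode.
; OnRep_Player_Data is empty, with its color material assignment left unconnected.
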(event `ChangeScore`
  (params (Team1Score :type Integer) (Team2Score :type Integer))
  (`/Game/HUD/BP_HUD.ChangeScoreUI` (`self.As BP HUD`) Team1Score Team2Score))

(event `MatchState`
  (params (Index :type Integer))
  (`/Game/HUD/BP_HUD.EndMatchWindow` (`self.As BP HUD`) Index))

(event `Draw`
  (bind _asbp_field_player_controller (cast `/Game/Blueprints/BP_FieldPlayerController` (`self.GetController`)))
  (bind _asbp_hud (cast `/Game/HUD/BP_HUD` (`PlayerController.GetHUD` _asbp_field_player_controller))
    (:`then`
      (bind _output_get (set `self.As BP HUD` _asbp_hud))
      (`/Game/HUD/BP_HUD.DrawUI` _output_get _asbp_field_player_controller))
    (:`CastFailed`
      (`KismetSystemLibrary.PrintString` "Hello"))))

(event `self.UI_DrawUI`
  (params (PlayerController :type "FieldPlayerController Object Reference"))
  (`self.Draw`))

(event `PlayerSpawned`
  (bind _asbp_ping_pong_game_mode (cast `/Game/Blueprints/BP_PingPongGameMode` (`GameplayStatics.GetGameMode`)))
  (`/Game/Blueprints/BP_PingPongGameMode.PlayerSpawned` _asbp_ping_pong_game_mode))

(fn `OnRep_Player_Data`)

(fn `UserConstructionScript`)