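; BP_Gate is a goal for the ping-pong game that registers scores and resets the ball.
; When a BP_Ball overlaps its Box, the Goal event reports its GoalTeam to BP_PingPong_GameMode through OnBallScore.
; It then spawns a replacement ball at the first TargetPoint found in the level, keeping the old ball's height, and destroys the old one.
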(event `self.Box.OnComponentBeginOverlap`
  (params (OverlappedComponent :type "PrimitiveComponent Object Reference") (OtherActor :type "Actor Object Reference") (OtherComp :type "PrimitiveComponent Object Reference") (OtherBodyIndex :type Integer) (bFromSweep :type Boolean) (SweepResult :type "HitResult Structure (by ref)"))
  (cast `/Game/Blueprints/BP_Ball` OtherActor)
  (`self.Goal` OtherActor))

(event `Goal`
  (params (Actor :type "Actor Object Reference"))
  (bind (_returnvalue_x _returnvalue_y _returnvalue_z) (`KismetMathLibrary.BreakVector` (`self.K2_GetActorLocation` Actor)))
  (bind _asbp_ping_pong_game_mode (cast `/Game/Blueprints/BP_PingPong_GameMode` (`GameplayStatics.GetGameMode`)))
  (`PingPongGameMode.OnBallScore` _asbp_ping_pong_game_mode (`self.GoalTeam`))
  (bind _outactors (`GameplayStatics.GetAllActorsOfClass` "/Script/Engine.TargetPoint"))
  (`/Engine/EditorBlueprintResources/StandardMacros.IsValid` Actor
    (:`Is Valid`
      (bind _returnvalue (`self.GetTransform` (`|GetArrayItem` _outactors)))
      (`|SpawnActorFromClass` "/Game/Blueprints/BP_Ball.BP_Ball_C" (`KismetMathLibrary.MakeTransform` (`KismetMathLibrary.MakeVector` (.x (.location _returnvalue)) (.y (.location _returnvalue)) _returnvalue_z)) "AdjustIfPossibleButAlwaysSpawn" "MultiplyWithRoot" null null)
      (`self.K2_DestroyActor` Actor))))

(fn `UserConstructionScript`)