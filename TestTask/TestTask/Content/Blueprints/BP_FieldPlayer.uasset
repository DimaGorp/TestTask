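; BP_FieldPlayer is a player Blueprint, apparently for a ping pong game, that manages the on-screen score and match-state UI.
; DrawUI creates a UMG_PlayerScore widget, stores it as PlayerUI and adds it to the viewport.
; UI-prefixed events forward to internal events that set both team scores on the widget or switch its windows by match-state index.
; BeginPlay is empty, and a game mode cast is left unconnected.
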(event `self.ReceiveBeginPlay`)

(event `self.UI_DrawUI`
  (`self.DrawUI` null))

(event `DrawUI`
  (params (OwningPlayer :type "PlayerController Object Reference"))
  (bind _returnvalue (`|CreateWidget` "/Game/HUD/UMG_PlayerScore.UMG_PlayerScore_C" OwningPlayer))
  (bind _output_get (set `self.PlayerUI` _returnvalue))
  (`UserWidget.AddToViewport` _output_get 0))

(event `ChangeScoreUI`
  (params (Team1Score :type Integer) (Team2Score :type Integer))
  (bind _playerui (`self.PlayerUI`))
  (`|ExecutionSequence`
    (:`then_0`
      (set `/Game/HUD/UMG_PlayerScore.Team1Score` Team1Score _playerui))
    (:`then_1`
      (set `/Game/HUD/UMG_PlayerScore.Team2Score` Team2Score _playerui))))

(event `self.UI_MatchState`
  (params (index :type Integer))
  (`self.EndMatchWindow` index))

(event `self.UI_ChangeScore`
  (params (team1_score :type Integer) (team2_score :type Integer))
  (`self.ChangeScoreUI` team1_score team2_score))

(event `EndMatchWindow`
  (params (Index :type Integer))
  (`/Game/HUD/UMG_PlayerScore.Switch Windows` (`self.PlayerUI`) Index))

(fn `UserConstructionScript`)