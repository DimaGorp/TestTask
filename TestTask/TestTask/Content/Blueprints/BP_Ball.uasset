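; BP_Ball is a physics-driven ball that launches itself and reacts to hits from field players.
; On BeginPlay it picks a random diagonal direction in the XY plane and applies it to Sphere1 as a velocity-change impulse.
; Hits from BP_FieldPlayer add a small impulse on X and Y, with both signs chosen by the ball's X velocity alone.
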(event `self.ReceiveBeginPlay`
  (bind _returnvalue (`KismetMathLibrary.SelectFloat` -1.0 1.0 (`KismetMathLibrary.RandomBool`)))
  (bind _output_get (set `self.Valocity` (`KismetMathLibrary.MakeVector` _returnvalue _returnvalue)))
  (`PrimitiveComponent.AddImpulse` (`self.Sphere1`) (* _output_get 1000.0) "None" true))

(event `self.ReceiveHit`
  (params (MyComp :type "PrimitiveComponent Object Reference") (Other :type "Actor Object Reference") (OtherComp :type "PrimitiveComponent Object Reference") (bSelfMoved :type Boolean) (HitLocation :type "Vector Structure") (HitNormal :type "Vector Structure") (NormalImpulse :type "Vector Structure") (Hit :type "HitResult Structure (by ref)"))
  (bind _returnvalue (`KismetMathLibrary.SelectFloat` 10.0 -10.0 (> (.x (`SceneComponent.GetComponentVelocity` (`self.Sphere1`))) 1.0)))
  (cast `/Game/Blueprints/BP_FieldPlayer` Other)
  (`PrimitiveComponent.AddImpulse` (`self.Sphere1`) (`KismetMathLibrary.MakeVector` _returnvalue _returnvalue) "None" false))

(fn `UserConstructionScript`)